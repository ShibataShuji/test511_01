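; BP_Saku is a fence (saku) actor that opens by rising while shrinking vertically.
; A timeline started at BeginPlay moves it up and reduces its Z scale each update while OpenFlag is set, until near a fixed height above its start.
; ToggleOpenFlag changes the flag through a FlipFlop with only the A branch wired, so only alternate calls act.
; No closing motion exists.
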(event EventBeginPlay
  (bind _returnvalue (Transformation|GetActorLocation))
  (Variables|Default|SetOriginVec (Transformation|GetActorLocation))
  (Timeline|タイムライン PlayFromStart
    (:Update
      (if (Variables|Default|GetOpenFlag)
        (if (not (Utilities|Operators|EqualEqual (Transformation|GetActorLocation) (Math|Vector|MakeVector (.x (Variables|Default|GetOriginVec)) (.y (Variables|Default|GetOriginVec)) (+ (.z (Variables|Default|GetOriginVec)) 1.9e+02)) 5.0))
          (Transformation|SetActorLocation (Math|Vector|MakeVector (.x _returnvalue) (.y _returnvalue) (+ (.z _returnvalue) 3.0)) false false)
          (Transformation|SetActorScale3D (Math|Vector|MakeVector 1.0 1.0 (- (.z (Transformation|GetActorScale3D)) 0.015))))))))

(fn ConstructionScript)

(fn ToggleOpenFlag
  (bind _isa (Utilities|FlowControl|FlipFlop)
    (:A
      (Variables|Default|SetOpenFlag (!= (Variables|Default|GetOpenFlag) _isa)))))