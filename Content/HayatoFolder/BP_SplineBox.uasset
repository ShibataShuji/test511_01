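; Actor that moves along a path supplied by a referenced spline actor.
; On BeginPlay it snaps to the transform the spline actor returns for its Distance with zero speed.
; Each Tick it passes Distance and frame-scaled Speed to the spline actor's GetSplineTransform and applies the returned transform without sweep.
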(event EventBeginPlay
  (bind _transform (Default|GetSplineTransform (Variables|Default|GetSplineActor) (Variables|Default|GetDistance) 0.0))
  (Transformation|SetActorTransform _transform))

(event Collision|EventActorBeginOverlap
  (params (OtherActor :type Actor%20Object%20Reference)))

(event EventTick
  (params (DeltaSeconds :type Float%20%28single-precision%29))
  (bind _transform (Default|GetSplineTransform (Variables|Default|GetSplineActor) (Variables|Default|GetDistance) (* DeltaSeconds (Variables|Default|GetSpeed))))
  (Transformation|SetActorTransform _transform))

(fn ConstructionScript)