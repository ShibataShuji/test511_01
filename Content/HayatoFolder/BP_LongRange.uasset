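; Long-range attacker actor that periodically fires BP_Bullet, apparently aimed at the player.
; A timeline serves as a cooldown clock, restarting once it passes ActionCoolTime and triggering Attack after a random delay of up to two seconds.
; Attack sets rotation through helper functions, whose look-at interpolation nodes are unconnected, then spawns a yaw-offset bullet carrying the shooter's location for reflection.
; It also caches a BP_ReflectBox reference and prints the timer for debugging.
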(event Custom|Attack
  (bind _returnvalue (Transformation|GetActorLocation))
  (Utilities|FlowControl|Sequence
    (:then_0
      (Transformation|SetActorRotation (|SetRotationZOnly) :!pinned true) ; プレイヤーの方を向かせてるよ
      (Variables|Default|SetAttackRotation (|SetRotation)))
    (:then_1
      (bind _returnvalue_2 (Game|SpawnActorfromClass "/Game/HayatoFolder/BP_Bullet.BP_Bullet_C" (Math|Transform|MakeTransform (Math|Vector|MakeVector (.x _returnvalue) (.y _returnvalue) (.z _returnvalue)) (Math|Rotator|MakeRotator (.roll (Variables|Default|GetAttackRotation)) (.pitch (Variables|Default|GetAttackRotation)) (+ (.yaw (Variables|Default|GetAttackRotation)) 9e+01)) "1.000000,1.000000,1.000000") "Undefined" 0 0 0 :!pinned true)) ; 弾撃つよ
      (Variables|/Game/HayatoFolder/BP_Bullet.BP_Bullet_C|SetOwnerActorLocation _returnvalue_2 (Transformation|GetActorLocation)) ; 弾を跳ね返した時用の変数
    )))

(event EventBeginPlay
  (Utilities|FlowControl|Sequence
    (:then_0
      ;[1 1 1] プレイヤーの取得
      (Variables|Default|SetAs%20BP%20Player (.AsBP%20Player (Utilities|Casting|CastToBP_Player (Game|GetPlayerCharacter 0)))))
    (:then_1
      (bind _新規track_0 (Timeline|999sTimeLine PlayFromStart)
        (:Update
          (Development|PrintString (Utilities|String|ToString(Float) _新規track_0) true true "(R=0.000000,G=0.660000,B=1.000000,A=1.000000)" 0.01)
          (if (< (Variables|Default|GetActionCoolTime) _新規track_0)
            (Utilities|FlowControl|Sequence
              (:then_0
                (Timeline|999sTimeLine PlayFromStart))
              (:then_1
                (Utilities|FlowControl|Delay (Math|Random|RandomFloatinRange 0.0 2.0))
                (CallFunction|Attack)))))))
    (:then_2
      (bind _returnvalue (Actor|GetActorOfClass "/Game/HayatoFolder/BP_ReflectBox.BP_ReflectBox_C"))
      (Variables|Default|SetAsReflectBox _returnvalue))))

(fn ConstructionScript)