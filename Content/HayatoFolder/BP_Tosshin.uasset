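; BP_Tosshin is an actor that performs a repeating charge (tosshin) attack toward the player.
; Attack takes one interpolated yaw step toward the player, then a timeline moves the actor along its forward vector, switching from wind-up speed to rush speed by elapsed time.
; After the rush and a cooldown it sets a finish flag, which a second timeline polls to attack again.
; The 1 key also triggers Attack directly.
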(event Custom|Attack
  (Utilities|FlowControl|Sequence
    (:then_0
      (Variables|Default|SetMoveFinishFlag false)
      (Transformation|SetActorRotation (Math|Interpolation|RInterpTo (Math|Rotator|MakeRotator 0.0 0.0 (.yaw (Transformation|GetActorRotation))) (Math|Rotator|MakeRotator 0.0 0.0 (.yaw (Math|Rotator|FindLookatRotation (Transformation|GetActorLocation) (Transformation|GetActorLocation (Variables|Default|GetAs%20BP%20Player))))) (Utilities|Time|GetWorldDeltaSeconds) 0.0) :!pinned true) ; プレイヤーの方を向かせてるよ
    )
    (:then_1
      (bind _新規track_0 (Timeline|タイムライン PlayFromStart)
        (:Update
          (Utilities|FlowControl|Sequence
            (:then_0
              (Transformation|AddActorWorldOffset (* (Transformation|GetActorForwardVector) (Variables|Default|GetMoveSpeed))))
            (:then_1
              ;[1 1 1] チャージ時間が終わったら、突進開始
              (if (and (> _新規track_0 (Variables|Default|GetChargeTime)) (<= _新規track_0 (Variables|Default|GetTosshinTime)))
                (Variables|Default|SetMoveSpeed (Variables|Default|GetTosshinSpeed))))
            (:then_2
              ;[1 1 1] 突進が終わる処理(今は時間で終わらせてるけど、「なにかにぶつかったら」とかになるかな)
              (if (> _新規track_0 (Variables|Default|GetTosshinTime))
                (Variables|Default|SetMoveSpeed (Math|Interpolation|FInterpTo (Variables|Default|GetTosshinSpeed) (Variables|Default|GetChargeSpeed) (Utilities|Time|GetWorldDeltaSeconds) 5e+01))
                (Utilities|FlowControl|Delay (Variables|Default|GetActionCoolTime))
                (Variables|Default|SetMoveFinishFlag true)
                (Variables|Default|SetMoveSpeed (Variables|Default|GetChargeSpeed))
                (Timeline|タイムライン Stop)))))))))

(event EventBeginPlay
  (Utilities|FlowControl|Sequence
    (:then_0
      ;[1 1 1] プレイヤーの取得
      (Variables|Default|SetAs%20BP%20Player (.AsBP%20Player (Utilities|Casting|CastToBP_Player (Game|GetPlayerCharacter 0)))))
    (:then_1
      (Utilities|FlowControl|DelayUntilNextTick)
      (Timeline|タイムライン_0 PlayFromStart
        (:Update
          (if (Variables|Default|GetMoveFinishFlag)
            (CallFunction|Attack)
            (Timeline|タイムライン_0 PlayFromStart)))))))

(event Input|KeyboardEvents|1
  (params (Key :type Key%20Structure :default "None"))
  (:Pressed
    (CallFunction|Attack)))

(fn ConstructionScript)