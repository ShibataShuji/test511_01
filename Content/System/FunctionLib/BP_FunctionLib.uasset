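; Function library for screen fades, with one function to start a fade and one to poll its completion.
; SetFade clears the game instance's FadeFinish flag, adds a new WBP_Fade widget to the viewport and sets its duration, alpha range and signed per-second delta for Forward or Reverse.
; FadeFinish reads that flag as a one-shot signal, resetting it whenever it returns true.
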(fn SetFade
  (params (Duration :type Float%20%28double-precision%29) (Selection :type EUMGSequencePlayMode%20Enum :default "Forward"))
  (Variables|/Game/System/GameInstance/BP_GameInstanece.BP_GameInstanece_C|SetFadeFinish (.AsBP%20Game%20Instanece (Utilities|Casting|CastToBP_GameInstanece (Game|GetGameInstance))) false)
  (LocalVariables|SetDulation Duration)
  (bind _returnvalue (UserInterface|CreateWidget "/Game/UI/WBP_Fade.WBP_Fade_C"))
  (bind _output_get (LocalVariables|SetWBP_Fade _returnvalue))
  (UserInterface|Viewport|AddtoViewport _output_get 10)
  (Variables|/Game/UI/WBP_Fade.WBP_Fade_C|SetDuration _output_get (LocalVariables|GetDulation))
  (switch Utilities|FlowControl|Switch|SwitchonEUMGSequencePlayMode Selection
    (:Forward
      (Variables|/Game/UI/WBP_Fade.WBP_Fade_C|SetFromAlpha (LocalVariables|GetWBP_Fade) 0.0)
      (bind _output_get_2 (Variables|/Game/UI/WBP_Fade.WBP_Fade_C|SetToAlpha (LocalVariables|GetWBP_Fade) 1.0))
      (Variables|/Game/UI/WBP_Fade.WBP_Fade_C|SetDeltaAlpha (LocalVariables|GetWBP_Fade) (/ _output_get_2 (LocalVariables|GetDulation))))
    (:Reverse
      (bind _output_get_3 (Variables|/Game/UI/WBP_Fade.WBP_Fade_C|SetFromAlpha (LocalVariables|GetWBP_Fade) 1.0))
      (Variables|/Game/UI/WBP_Fade.WBP_Fade_C|SetToAlpha (LocalVariables|GetWBP_Fade) 0.0)
      (Variables|/Game/UI/WBP_Fade.WBP_Fade_C|SetDeltaAlpha (LocalVariables|GetWBP_Fade) (* (/ _output_get_3 (LocalVariables|GetDulation)) -1.0))))
  (return))

(fn FadeFinish
  (if (Variables|/Game/System/GameInstance/BP_GameInstanece.BP_GameInstanece_C|GetFadeFinish (.AsBP%20Game%20Instanece (Utilities|Casting|CastToBP_GameInstanece (Game|GetGameInstance))))
    (Variables|/Game/System/GameInstance/BP_GameInstanece.BP_GameInstanece_C|SetFadeFinish (.AsBP%20Game%20Instanece (Utilities|Casting|CastToBP_GameInstanece (Game|GetGameInstance))) false)
    (return true)
    (else
      (return false))))