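; BP_SceneChanged is a trigger that moves the player between streamed sub-level areas on overlap.
; It builds zero-padded area names from Path and the current level name, then requests a blocking load of NextArea.
; It teleports the player to the BP_SceneChangePosition tagged with that area and TagNumber.
; It then unloads NowArea, though only the branch for area numbers below 10 reaches the unload.
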(event OnComponentBeginOverlap(flag)
  (params (OverlappedComponent :type Primitive%20Component%20Object%20Reference) (OtherActor :type Actor%20Object%20Reference) (OtherComp :type Primitive%20Component%20Object%20Reference) (OtherBodyIndex :type Integer) (bFromSweep :type Boolean) (SweepResult :type Hit%20Result%20Structure%20%28by%20ref%29))
  (bind _nowarea (Variables|エリア|GetNowArea))
  (bind _nextarea (Variables|エリア|GetNextArea))
  (bind _nextarea_2 (Variables|エリア|GetNextArea))
  (Utilities|Casting|CastToBP_Player OtherActor)
  (Utilities|FlowControl|Sequence
    (:then_0
      ;[0.3153 0.9582 1] Load処理
      (if (< _nextarea_2 10)
        (Variables|エリア|SetAreaNumString (Utilities|String|StringToName (Utilities|String|Append "0" (Utilities|String|ToString(Integer) _nextarea_2))))
        (else
          (Variables|エリア|SetAreaNumString (Utilities|String|StringToName (Utilities|String|BuildString(Integer) "" "" _nextarea_2)))))
      (bind _returnvalue (Game|GetCurrentLevelName true))
      (bind _output_get (Variables|エリア|SetLoadName (Utilities|String|StringToName (Utilities|String|Append (Utilities|String|ToString(Name) (Variables|エリア|GetPath)) _returnvalue "/" _returnvalue "_Area" (Utilities|String|ToString(Name) (Variables|エリア|GetAreaNumString))))))
      (Development|PrintString (Utilities|String|Append "Load" (Utilities|String|ToString(Name) _output_get)))
      (Game|LoadStreamLevel(byName) _output_get true true))
    (:then_1
      (Variables|シーン遷移ポジション|SetTagNumString (Utilities|String|StringToName (Utilities|String|BuildString(Integer) "" "" (Variables|シーン遷移ポジション|GetTagNumber))))
      (if (< _nextarea 10)
        (Variables|シーン遷移ポジション|SetTagAreaNum (Utilities|String|StringToName (Utilities|String|Append "0" (Utilities|String|ToString(Integer) _nextarea))))
        (else
          (Variables|シーン遷移ポジション|SetTagAreaNum (Utilities|String|StringToName (Utilities|String|BuildString(Integer) "" "" _nextarea)))))
      (bind _output_get_2 (Variables|シーン遷移ポジション|SetTagName (Utilities|String|StringToName (Utilities|String|Append "Area" (Utilities|String|ToString(Name) (Variables|シーン遷移ポジション|GetTagAreaNum)) "_" (Utilities|String|ToString(Name) (Variables|シーン遷移ポジション|GetTagNumString))))))
      (Development|PrintString (Utilities|String|ToString(Name) _output_get_2))
      (bind _outactors (Actor|GetAllActorsOfClass "/Game/System/SceneChange/BP_SceneChangePosition.BP_SceneChangePosition_C"))
      (bind _array_element (Utilities|Array|ForEachLoopwithBreak _outactors :!label _label)
        (:LoopBody
          (if (Actor|ActorHasTag _array_element (Variables|シーン遷移ポジション|GetTagName))
            (Utilities|FlowControl|Sequence
              (:then_0
                (goto _label Break))
              (:then_1
                (bind _output_get_3 (Variables|シーン遷移ポジション|SetSceneChangePosition (Transformation|GetActorLocation _array_element)))
                (Development|PrintString (Utilities|String|ToString(Vector) _output_get_3))
                (Transformation|SetActorLocation (.AsBP%20Player (Utilities|Casting|CastToBP_Player (Game|Player|GetPlayerPawn 0))) (Variables|シーン遷移ポジション|GetSceneChangePosition) false false)))))))
    (:then_2
      ;[1 0.9918 0.1314] UnLoad処理
      (if (< _nowarea 10)
        (bind _output_get_4 (Variables|エリア|SetAreaNumString (Utilities|String|StringToName (Utilities|String|Append "0" (Utilities|String|ToString(Integer) _nowarea)))))
        (bind _returnvalue_2 (Game|GetCurrentLevelName true))
        (Variables|エリア|SetUnLoadName (Utilities|String|StringToName (Utilities|String|Append (Utilities|String|ToString(Name) (Variables|エリア|GetPath)) _returnvalue_2 "/" _returnvalue_2 "_Area" (Utilities|String|ToString(Name) _output_get_4))))
        (Development|PrintString "Unload")
        (Game|UnloadStreamLevel(byName) (Variables|エリア|GetUnLoadName) true)
        (else
          (Variables|エリア|SetAreaNumString (Utilities|String|StringToName (Utilities|String|BuildString(Integer) "" "" _nowarea))))))))

(fn ConstructionScript)