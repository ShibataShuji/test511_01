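; AI controller for the Rush enemy type that runs behavior tree BT_5 on BeginPlay.
; Its AI perception updates drive the TargetActor blackboard key.
; Sensing the player calls the pawn's BP_AIEnemy found-target action, then stores the player as target.
; Losing the player, or any perception update from another actor, clears the key.
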(event OnTargetPerceptionUpdated(AIPerception)
  (params (Actor :type Actor%20Object%20Reference) (Stimulus :type AI%20Stimulus%20Structure))
  (if (== Actor (Game|GetPlayerCharacter 0))
    (if (.bSuccessfullySensed (Utilities|Struct|BreakAIStimulus Stimulus))
      ;[1 1 1] 見つけた瞬間だよっていうのを伝える
      (bind _asbp_aienemy (Utilities|Casting|CastToBP_AIEnemy (Pawn|GetControlledPawn)))
      (Default|ActionattheMomentOfFindingtheTarget _asbp_aienemy)
      ;[1 1 1] プレイヤーをセットする
      (AI|Components|Blackboard|SetValueasObject (Variables|Default|GetBlackboard) (Utilities|Name|MakeLiteralName "TargetActor") Actor)
      (else
        ;[1 1 1] nullをセットする
        (AI|Components|Blackboard|SetValueasObject (Variables|Default|GetBlackboard) (Utilities|Name|MakeLiteralName "TargetActor") 0 :!label _label)))
    (else
      (goto _label))))

(event EventBeginPlay
  (AI|RunBehaviorTree "/Game/MyContents/Enemy/05_Rush/BT_5.BT_5"))

(event EventTick
  (params (DeltaSeconds :type Float%20%28single-precision%29)))

(fn ConstructionScript)