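; Rush enemy AI child Blueprint that drives its behavior through Blackboard keys, teleporting to its home location and clearing target-in-sight on start.
; Parent behavior overrides call matching events: with no target in sight it runs MoveEvent and writes MoveLocation as the target.
; Spotting a target briefly sets the AI-stop flag.
; In-range and out-of-range actions only print debug text, while knockback and guard defer to the parent.
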(event Custom|Action%20to%20be%20taken%20out%20of%20range%20Event
  ;[1 1 1] 範囲外でとる行動
  (Development|PrintString "範囲外でとる行動"))

(event Custom|Action%20to%20be%20taken%20within%20range%20Event
  ;[1 1 1] 範囲内でとる行動
  (Development|PrintString "範囲内でとる行動"))

(event Custom|Init%20actor%20state
  ;[1 1 1] 初期化
  (Utilities|FlowControl|Sequence
    (:then_0
      (Transformation|SetActorLocation (Variables|Default|GetHome%20Location) false true))
    (:then_1
      (AI|Components|Blackboard|SetValueasBool (AI|GetBlackboard 0) (Variables|Default|GetBB_TargetInSight) false))))

(event Custom|Action%20when%20the%20target%20is%20not%20in%20sight%20Event
  ;[1 1 1] ターゲットを視認していないときの行動
  (Development|PrintString "ターゲットを視認していないときの行動")
  (CallFunction|MoveEvent)
  (AI|Components|Blackboard|SetValueasVector (AI|GetBlackboard 0) (Variables|Default|GetBB_TargetLocation) (Variables|Default|GetMove%20Location)))

(event Custom|Action%20at%20the%20moment%20of%20finding%20the%20target%20Event
  ;[1 1 1] ターゲットを見つけた瞬間の行動
  (Development|PrintString "ターゲットを見つけた瞬間の行動")
  (AI|Components|Blackboard|SetValueasBool (AI|GetBlackboard 0) (Variables|Default|GetBB_AIstops) true)
  (Utilities|FlowControl|Delay 1.0)
  (AI|Components|Blackboard|SetValueasBool (AI|GetBlackboard 0) (Variables|Default|GetBB_AIstops) false))

(event EventBeginPlay
  (|CallParentFunction)
  (CallFunction|InitActorState))

(event EventTick
  (params (DeltaSeconds :type Float%20%28single-precision%29)))

(fn ConstructionScript
  (|CallParentFunction))

(fn Knockback
  (params (Knockback%20Direction :type Vector :default "0, 0, 0") (Knockback%20Strength :type Float%20%28double-precision%29) (Knockback%20Strength%20Z :type Float%20%28double-precision%29))
  (|CallParentFunction Knockback%20Direction Knockback%20Strength Knockback%20Strength%20Z))

(fn GuardStart
  (|CallParentFunction))

(fn GuardEnd
  (|CallParentFunction))

(fn ActionwhentheTargetIsNotinSight
  (|CallParentFunction)
  (CallFunction|ActionwhentheTargetIsNotinSightEvent)
  (Variables|Default|GetMove%20Spline
    (:then
      (return true))
    (:else
      (return true))))

(fn ActionattheMomentOfFindingtheTarget
  (|CallParentFunction)
  (CallFunction|ActionattheMomentOfFindingtheTargetEvent))

(fn ActiontobeTakenOutOfRange
  (|CallParentFunction)
  (CallFunction|ActiontobeTakenOutOfRangeEvent))

(fn ActiontobeTakenWithinRange
  (|CallParentFunction)
  (CallFunction|ActiontobeTakenWithinRangeEvent))