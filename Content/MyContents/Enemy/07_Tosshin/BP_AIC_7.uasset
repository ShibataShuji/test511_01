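; AI controller for enemy 07 (Tosshin) that runs BT_7 and tracks the player through AIPerception.
; First sighting notifies the BP_AIEnemy pawn and sets the TargetActor blackboard key.
; After sight is lost, 30sTimeline polls until the player is re-sensed or farther than 1500 units, which triggers the loss action and clears the key.
; A perception update from any other actor also clears TargetActor, leaving the detection flag unchanged.
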(event OnTargetPerceptionUpdated(AIPerception)
  (params (Actor :type Actor%20Object%20Reference) (Stimulus :type AI%20Stimulus%20Structure))
  (bind _returnvalue (Game|GetPlayerCharacter 0))
  (if (== Actor _returnvalue)
    (if (.bSuccessfullySensed (Utilities|Struct|BreakAIStimulus Stimulus))
      (Utilities|FlowControl|Sequence
        (:then_0
          (Variables|Default|SetLost%20Sight false))
        (:then_1
          (if (not (Variables|Default|GetCurrent%20Status))
            ;[1 1 1] 見つけた瞬間だよっていうのを伝える
            (Variables|Default|SetCurrent%20Status true)
            (bind _asbp_aienemy (Utilities|Casting|CastToBP_AIEnemy (Pawn|GetControlledPawn)))
            (Default|ActionattheMomentOfFindingtheTarget _asbp_aienemy)
            ;[1 1 1] プレイヤーをセットする
            (AI|Components|Blackboard|SetValueasObject (Variables|Default|GetBlackboard) (Utilities|Name|MakeLiteralName "TargetActor") Actor))))
      (else
        (Utilities|FlowControl|Sequence
          (:then_0
            (Variables|Default|SetLost%20Sight true))
          (:then_1
            (Timeline|30sTimeline PlayFromStart
              (:Update
                (if (Variables|Default|GetLost%20Sight)
                  (if (> (Math|Vector|VectorLength (- (Transformation|GetActorLocation _returnvalue) (Transformation|GetActorLocation (Pawn|GetControlledPawn)))) 1.5e+03)
                    (Utilities|FlowControl|Sequence
                      (:then_0
                        (Timeline|30sTimeline Stop))
                      (:then_1
                        (if (Variables|Default|GetCurrent%20Status)
                          (Variables|Default|SetCurrent%20Status false)
                          ;[1 1 1] 見失った瞬間を伝える
                          (bind _asbp_aienemy_2 (Utilities|Casting|CastToBP_AIEnemy (Pawn|GetControlledPawn)))
                          (Default|ActionattheMomentOfLoss _asbp_aienemy_2)
                          ;[1 1 1] nullをセットする
                          (AI|Components|Blackboard|SetValueasObject (Variables|Default|GetBlackboard) (Utilities|Name|MakeLiteralName "TargetActor") 0 :!label _label)))))
                  (else
                    (Timeline|30sTimeline Stop)))))))))
    (else
      (goto _label))))

(event EventBeginPlay
  (AI|RunBehaviorTree "/Game/MyContents/Enemy/07_Tosshin/BT_7.BT_7"))

(event EventTick
  (params (DeltaSeconds :type Float%20%28single-precision%29)))

(fn ConstructionScript)