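; Charging AI enemy that rushes toward the player and knocks them back on contact.
; Parent AI hook overrides forward to events that pause and resume the AI through a Blackboard flag and timers as the target is found, lost or in range.
; In range, it turns toward the player and moves straight without pathfinding.
; Timeline-driven traces and checks end the charge on obstacle, player hit, arrival or timeout, then AI resumes after cooldown.
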(event Custom|Action%20at%20the%20moment%20of%20loss%20Event
  ;[1 1 1] ターゲットを見失ったかもしれない瞬間
  (Development|PrintString "ターゲットを見失ったかもしれない")
  (if (not (Variables|Default|GetIs%20Falling%20Actions))
    (CallFunction|StopsAIEvent)))

(event Custom|Trace%20Forward%20object
  (Timeline|タイムライン_2 PlayFromStart
    (:Update
      (bind _returnvalue (CallFunction|TraceFunctionForward 1.3 "TraceTypeQuery4" 17.0 "(R=0.000000,G=0.379607,B=1.000000,A=1.000000)" 1.0))
      (if (not _returnvalue)
        (Variables|Default|SetTosshinEndFlag true) ; 目の前に通れない場所があって終了
        (Development|PrintString "目の前に通れない場所があって終了" true true "(R=1.000000,G=0.000000,B=0.122032,A=1.000000)" 0.01)))))

(event Custom|Action%20to%20be%20taken%20out%20of%20range%20Event
  ;[1 1 1] 範囲外でとる行動
  (Development|PrintString "範囲外でとる行動"))

(event Custom|Action%20to%20be%20taken%20within%20range%20Event
  ;[1 1 1] 範囲内でとる行動
  (Development|PrintString "範囲内でとる行動")
  (CallFunction|StopsAIEvent)
  (CallFunction|AttackEvent))

(event Custom|Init%20actor%20state
  ;[0.542 0.8687 1 1 120] 初期化系
  ;;[1 1 1] 初期化
  (Utilities|FlowControl|Sequence
    (:then_0
      (Transformation|SetActorLocation (Variables|Default|GetHome%20Location) false true))
    (:then_1
      (AI|Components|Blackboard|SetValueasBool (AI|GetBlackboard 0) (Variables|Default|GetBB_TargetInSight) false)
      (AI|Components|Blackboard|SetValueasFloat (AI|GetBlackboard 0) (Variables|Default|GetBB_AttackRange) (Variables|Default|GetNext%20Attack%20Range))
      (AI|Components|Blackboard|SetValueasBool (AI|GetBlackboard 0) (Variables|Default|GetBB_UseMoveOutAttackRange) true))))

(event Custom|Start%20AI%20Delay%20Event
  (params (Time :type Float%20%28single-precision%29))
  ;[1 0.3991 0.963 1 120] Ai系
  (bind _returnvalue (Utilities|Time|SetTimerbyEvent (delegate Custom|Start%20AI%20Delay%20Event%20Sub) Time))
  (Variables|Default|SetStart%20AI%20Delay%20Event%20Timer _returnvalue))

(event Custom|Start%20AI%20Delay%20Event%20Sub
  ;[1 0.3991 0.963 1 120] Ai系
  (AI|Components|Blackboard|SetValueasBool (AI|GetBlackboard 0) (Variables|Default|GetBB_AIstops) false)
  (Development|PrintString "AIついたよ"))

(event Custom|Lost%20it%20completely%20Event
  ;[1 1 1] ターゲットを完全に見失った瞬間
  (Development|PrintString "完全に見失った")
  (if (not (Variables|Default|GetIs%20Falling%20Actions))
    (CallFunction|StartAIEvent)))

(event Custom|AttackEnd
  ;[1 1 1] 攻撃が終わる条件
  (Utilities|FlowControl|Sequence
    (:then_0
      (if (< (Math|Vector|VectorLength (- (Transformation|GetActorLocation) (Variables|Default|GetGoalLocation))) 5e+01)
        (Variables|Default|SetTosshinEndFlag true) ; 目的地と近くなって終了
        (Development|PrintString "目的地と近くなって終了" true true "(R=1.000000,G=0.000000,B=0.122032,A=1.000000)" 0.1)))))

(event Custom|TraceForwardObject_Short
  (Timeline|タイムライン_4 PlayFromStart
    (:Update
      (bind _outhit (CallFunction|TraceFunctionForward 0.0 "TraceTypeQuery4" 1.0 "(R=1.000000,G=0.000000,B=0.000000,A=1.000000)" 1.0))
      (if (.bSuccess (Utilities|Casting|CastToBP_Player (.HitActor (Collision|BreakHitResult _outhit))))
        (if (not (Variables|Default|GetTosshinEndFlag))
          (Variables|Default|SetTosshinEndFlag true) ; プレイヤーとぶつかって終了
          (Development|PrintString "プレイヤーとぶつかって終了" true true "(R=1.000000,G=0.000000,B=0.122032,A=1.000000)")
          (CallFunction|HitPlayerEvent (Transformation|GetActorForwardVector) 2e+03))))))

(event Custom|Hit%20Player%20Event
  (params (Hit%20Normal :type Vector) (Hit%20Strangth :type Float%20%28double-precision%29) (Hit%20Actor :type Actor%20Object%20Reference))
  (bind _asbp_player (Utilities|Casting|CastToBP_Player (Game|GetPlayerCharacter 0)))
  (Default|Knockback _asbp_player Hit%20Normal Hit%20Strangth 0.0))

(event Custom|Stops%20AI%20With%20Time%20Event
  (params (Stop%20time :type Float%20%28double-precision%29))
  (bind _start_ai_delay_event_timer (Variables|Default|GetStart%20AI%20Delay%20Event%20Timer))
  ;[1 0.3991 0.963 1 120] Ai系
  (Utilities|FlowControl|Sequence
    (:then_0
      (if (Utilities|Time|IsValidTimerHandle _start_ai_delay_event_timer)
        (if (Utilities|Time|IsTimerActivebyHandle _start_ai_delay_event_timer)
          (Utilities|Time|ClearandInvalidateTimerbyHandle _start_ai_delay_event_timer))))
    (:then_1
      (if (Utilities|Time|IsValidTimerHandle (Variables|Default|GetStop%20AI%20Timer))
        (if (Utilities|Time|IsTimerActivebyHandle (Variables|Default|GetStop%20AI%20Timer))
          ;;[1 1 1] 新しい値が残り時間より多かったら更新
          (if (> Stop%20time (Utilities|Time|GetTimerRemainingTimebyHandle (Variables|Default|GetStop%20AI%20Timer)))
            (AI|Components|Blackboard|SetValueasBool (AI|GetBlackboard 0) (Variables|Default|GetBB_AIstops) true :!label _label)
            (bind _returnvalue (Utilities|Time|SetTimerbyEvent (delegate Custom|Stops%20AI%20Event%20Sub) Stop%20time))
            (Variables|Default|SetStop%20AI%20Timer _returnvalue))
          (else
            (goto _label)))
        (else
          (goto _label))))))

(event Custom|Attack%20Event
  (Development|PrintString "突進開始ィィィィ！！！" true true "(R=1.000000,G=0.000000,B=0.035882,A=1.000000)")
  (Variables|Default|SetTosshinEndFlag false)
  (Transformation|SetActorRotation (Math|Interpolation|RInterpTo (Math|Rotator|MakeRotator 0.0 0.0 (.yaw (Transformation|GetActorRotation))) (Math|Rotator|MakeRotator 0.0 0.0 (.yaw (Math|Rotator|FindLookatRotation (Transformation|GetActorLocation) (Transformation|GetActorLocation (Game|GetPlayerCharacter 0))))) (Utilities|Time|GetWorldDeltaSeconds) 0.0))
  (Utilities|FlowControl|DelayUntilNextTick)
  (Utilities|FlowControl|Sequence
    (:then_0
      (Variables|Default|SetGoalLocation (+ (* (Transformation|GetActorForwardVector) (Variables|Default|GetGoalPoint)) (Transformation|GetActorLocation)))
      (Collision|SphereTraceByChannel (Variables|Default|GetGoalLocation) (Variables|Default|GetGoalLocation) 5e+01 "TraceTypeQuery1" false 0 "ForDuration" true "(R=1.000000,G=0.000000,B=0.000000,A=1.000000)" "(R=0.000000,G=0.061501,B=1.000000,A=1.000000)") ; 突進の最終到達点のチェック
    )
    (:then_1
      (AI|Navigation|MovetoLocation (AI|GetAIController self) (Variables|Default|GetGoalLocation) 5e+01 true false false true 0))
    (:then_2
      (CallFunction|TraceForwardObject)
      (CallFunction|TraceForwardObjectShort))
    (:then_3
      ;[1 1 1] 突進の終わりの処理
      (Timeline|タイムライン_3 PlayFromStart
        (:Update
          (Utilities|FlowControl|Sequence
            (:then_0
              (CallFunction|AttackEnd) ; 各種条件でTosshinEndFlagをtrueにする
            )
            (:then_1
              (if (Variables|Default|GetTosshinEndFlag)
                (Class|NavMovementComponent|StopActiveMovement (Variables|Character|GetCharacterMovement) :!label _label)
                (CallFunction|StartAIDelayEvent (Variables|Default|GetAttack%201%20CoolTime)) ; AIの再開
              ))))
        (:Finished
          (if (not (Variables|Default|GetTosshinEndFlag))
            (Variables|Default|SetTosshinEndFlag true) ; 時間経過で終了
            (Development|PrintString "時間経過で終了" true true "(R=1.000000,G=0.000000,B=0.122032,A=1.000000)")
            (goto _label)))))))

(event Custom|Stops%20AI%20Event%20Sub
  ;[1 0.3991 0.963 1 120] Ai系
  (AI|Components|Blackboard|SetValueasBool (AI|GetBlackboard 0) (Variables|Default|GetBB_AIstops) false))

(event Custom|Start%20AI%20Event
  ;[1 0.3991 0.963 1 120] Ai系
  (AI|Components|Blackboard|SetValueasBool (AI|GetBlackboard 0) (Variables|Default|GetBB_AIstops) false)
  (Development|PrintString "AIついたよ"))

(event Custom|Stops%20AI%20Event
  (bind _start_ai_delay_event_timer (Variables|Default|GetStart%20AI%20Delay%20Event%20Timer))
  ;[1 0.3991 0.963 1 120] Ai系
  (Utilities|FlowControl|Sequence
    (:then_0
      (if (Utilities|Time|IsValidTimerHandle _start_ai_delay_event_timer)
        (if (Utilities|Time|IsTimerActivebyHandle _start_ai_delay_event_timer)
          (Utilities|Time|ClearandInvalidateTimerbyHandle _start_ai_delay_event_timer))))
    (:then_1
      (AI|Components|Blackboard|SetValueasBool (AI|GetBlackboard 0) (Variables|Default|GetBB_AIstops) true))))

(event Custom|Falling%20Action%20Event
  ;[1 1 1] 落下開始した瞬間。モーションなどを再生し、落下させる
  (CallFunction|FallingActionNormal))

(event Custom|Action%20when%20the%20target%20is%20not%20in%20sight%20Event
  (bind _move_location (Variables|Default|GetMove%20Location))
  ;[1 1 1] ターゲットを視認していないときの行動
  (Development|PrintString "ターゲットを視認していないときの行動")
  (CallFunction|MoveEvent)
  (AI|Components|Blackboard|SetValueasVector (AI|GetBlackboard 0) (Variables|Default|GetBB_TargetLocation) _move_location)
  (Development|PrintString (Utilities|String|ToString(Vector) _move_location)))

(event Custom|Action%20at%20the%20moment%20of%20finding%20the%20target%20Event
  ;[1 1 1] ターゲットを見つけた瞬間の行動
  (if (Variables|Default|GetMay%20have%20lost%20Target)
    (Variables|Default|SetMay%20have%20lost%20Target false)
    (CallFunction|StartAIEvent)
    (Development|PrintString "ターゲットを再度見つけた")
    (else
      (Development|PrintString "ターゲットを見つけた瞬間の行動")
      (CallFunction|StopsAIwithTimeEvent 0.6)
      (CallFunction|RotateTowardtheTarget (Transformation|GetActorLocation (Game|GetPlayerCharacter 0)) 0.3))))

(event EventBeginPlay
  ;[0.542 0.8687 1 1 120] 初期化系
  (|CallParentFunction)
  (CallFunction|InitActorState))

(event EventTick
  (params (DeltaSeconds :type Float%20%28single-precision%29)))

(fn ConstructionScript
  (|CallParentFunction))

(fn Knockback
  (params (Knockback%20Direction :type Vector :default "0, 0, 0") (Knockback%20Strength :type Float%20%28double-precision%29) (Knockback%20Strength%20Z :type Float%20%28double-precision%29))
  (|CallParentFunction Knockback%20Direction Knockback%20Strength Knockback%20Strength%20Z))

(fn ActionwhentheTargetIsNotinSight
  (|CallParentFunction)
  (CallFunction|ActionwhentheTargetIsNotinSightEvent)
  (Variables|Default|GetMove%20Spline
    (:then
      (return true))
    (:else
      (return true))))

(fn ActionattheMomentOfFindingtheTarget
  (|CallParentFunction)
  (CallFunction|ActionattheMomentOfFindingtheTargetEvent))

(fn ActiontobeTakenOutOfRange
  (|CallParentFunction)
  (CallFunction|ActiontobeTakenOutOfRangeEvent))

(fn ActiontobeTakenWithinRange
  (|CallParentFunction)
  (CallFunction|ActiontobeTakenWithinRangeEvent))

(fn ActionattheMomentOfLoss
  (|CallParentFunction)
  (CallFunction|ActionattheMomentOfLossEvent))

(fn StopsAIwithTime
  (params (Stop%20time :type Float%20%28double-precision%29))
  (|CallParentFunction Stop%20time)
  (CallFunction|StopsAIwithTimeEvent Stop%20time))

(fn StartAI
  (|CallParentFunction)
  (CallFunction|StartAIEvent))

(fn StopsAI
  (|CallParentFunction)
  (CallFunction|StopsAIEvent))

(fn FallingAction
  (|CallParentFunction)
  (CallFunction|FallingActionEvent))

(fn StartAIDelay
  (params (Delay%20Time :type Float%20%28double-precision%29))
  (|CallParentFunction Delay%20Time)
  (CallFunction|StartAIDelayEvent Delay%20Time))

(fn HitPlayer
  (params (Hit%20Normal :type Vector :default "0, 0, 0") (Hit%20Strangth :type Float%20%28double-precision%29) (Hit%20Actor :type Actor%20Object%20Reference))
  (bind (_hit_normal_out _hit_strangth_out _hit_actor_out) (|CallParentFunction Hit%20Normal Hit%20Strangth Hit%20Actor))
  (CallFunction|HitPlayerEvent _hit_normal_out _hit_strangth_out _hit_actor_out)
  (return _hit_normal_out _hit_strangth_out _hit_actor_out))

(fn LostItCompletely
  (|CallParentFunction)
  (CallFunction|LostItCompletelyEvent))