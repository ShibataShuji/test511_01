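; Guard-type AI enemy Blueprint that carries out Attack and Guard actions signaled by its Behavior Tree.
; Each action sets Blackboard busy, interval and readiness keys, then restores them through long timelines used as cooldown and interval timers.
; Guard spawns a shield actor in front and turns the enemy toward the player until the timer ends and destroys it.
; Attack currently runs only its cooldown, with no damage or movement.
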(event Custom|Guard%20End%20Event)

(event Custom|Guard%20Start%20Event)

(event Custom|Change%20Battle%20State%20Event
  (params (BattleState :type BPE_BattleState_4%20Enum :default "NewEnumerator0")))

(event Custom|Receive%20Action%20Signal%20Event
  (params (BattleState :type BPE_BattleState_4%20Enum :default "NewEnumerator0"))
  ;[1 1 1] BTからアクション開始の信号が来る
  ;[1 1 1] 基本trueで来ることはないけど一応
  (if (not (Variables|Default|GetInAction))
    (Variables|Default|SetBattleState BattleState)
    ;[1 1 1] アクション中にする
    (Variables|Default|SetInAction true)
    (AI|Components|Blackboard|SetValueasBool (AI|GetBlackboard 0) (Variables|Default|GetBB_InAction) true)
    ;[1 1 1] アクションのインターバル中にする
    (AI|Components|Blackboard|SetValueasBool (AI|GetBlackboard 0) (Variables|Default|GetBB_DuringInterval) true)
    (switch Utilities|FlowControl|Switch|SwitchonBPE_BattleState_4 (Variables|Default|GetBattleState)
      (:NewEnumerator2
        (CallFunction|AttackEvent))
      (:NewEnumerator3
        (CallFunction|GuardEvent)))))

(event Custom|Attack%20Event
  (AI|Components|Blackboard|SetValueasBool (AI|GetBlackboard 0) (Variables|Default|GetBB_ReadyAttack) false)
  (Utilities|FlowControl|Sequence
    (:then_0)
    (:then_1
      (bind _elapsedtimes (Timeline|999sTimeLine_1 PlayFromStart)
        (:Update
          (if (> _elapsedtimes (Variables|Default|GetAttack%20Cool%20TIme))
            (Utilities|FlowControl|Sequence
              (:then_0
                (Timeline|999sTimeLine_1 Stop))
              (:then_1
                (Variables|Default|SetInAction false)
                (AI|Components|Blackboard|ClearValue (AI|GetBlackboard 0) (Variables|Default|GetBB_InAction))
                (AI|Components|Blackboard|SetValueasBool (AI|GetBlackboard 0) (Variables|Default|GetBB_ReadyAttack) true)
                (CallFunction|ActionIntervalEvent))
              (:then_2))))))))

(event Custom|Guard%20Event
  (bind _returnvalue (Transformation|GetActorTransform))
  (bind (_location _rotation) (Math|Transform|BreakTransform _returnvalue))
  (Development|PrintString "がーどかいし")
  (AI|Components|Blackboard|SetValueasBool (AI|GetBlackboard 0) (Variables|Default|GetBB_ReadyGuard) false)
  (Utilities|FlowControl|Sequence
    (:then_0
      (Variables|Default|SetOn%20Guard true)
      (bind _returnvalue_2 (Game|SpawnActorfromClass "/Game/MyContents/Weapon/Shield/BP_Weapon_Shield.BP_Weapon_Shield_C" (Math|Transform|MakeTransform (+ _location (* (Math|Vector|GetForwardVector _rotation) 5e+01)) _rotation) "AlwaysSpawn" 0 self 0))
      (Variables|Default|SetShieldActor _returnvalue_2))
    (:then_1
      (bind _elapsedtimes (Timeline|999sTimeLine_2 PlayFromStart)
        (:Update
          (if (> _elapsedtimes (Variables|Default|GetGuard%20Cool%20TIme))
            (Utilities|FlowControl|Sequence
              (:then_0
                (Timeline|999sTimeLine_2 Stop))
              (:then_1
                (Variables|Default|SetInAction false)
                (AI|Components|Blackboard|ClearValue (AI|GetBlackboard 0) (Variables|Default|GetBB_InAction))
                (AI|Components|Blackboard|SetValueasBool (AI|GetBlackboard 0) (Variables|Default|GetBB_ReadyGuard) true)
                (CallFunction|ActionIntervalEvent))
              (:then_2
                ;[1 1 1] 終了処理
                (Variables|Default|SetOn%20Guard false)
                (Actor|DestroyActor (Variables|Default|GetShieldActor))))
            (else
              ;[1 1 1] 行動中ルーループさせるようなものはここに書く
              (Transformation|SetActorRotation (Math|Rotator|FindLookatRotation (Transformation|GetActorLocation) (Transformation|GetActorLocation (Game|GetPlayerCharacter 0)))))))))))

(event Custom|Action%20Interval%20Event
  ;[1 1 1] アクションのインターバル時間処理
  (bind _elapsedtimes (Timeline|999sTimeLine_0 PlayFromStart)
    (:Update
      (if (> _elapsedtimes (Variables|Default|GetActionIntervalTIme))
        (Utilities|FlowControl|Sequence
          (:then_0
            (Timeline|999sTimeLine_0 Stop))
          (:then_1
            (AI|Components|Blackboard|SetValueasBool (AI|GetBlackboard 0) (Variables|Default|GetBB_DuringInterval) false)))))))

(event EventBeginPlay
  (|CallParentFunction)
  (AI|Components|Blackboard|SetValueasBool (AI|GetBlackboard 0) (Variables|Default|GetKey%20Name) true)
  (Class|BlackboardComponent|SetValueasInt (AI|GetBlackboard 0) (Variables|Default|GetBB_NumberofActions)))

(event Collision|EventActorBeginOverlap
  (params (OtherActor :type Actor%20Object%20Reference)))

(event EventTick
  (params (DeltaSeconds :type Float%20%28single-precision%29)))

(fn ConstructionScript
  (|CallParentFunction))

(fn Knockback
  (params (Knockback%20Direction :type Vector :default "0, 0, 0") (Knockback%20Strength :type Float%20%28double-precision%29) (Knockback%20Strength%20Z :type Float%20%28double-precision%29))
  (|CallParentFunction Knockback%20Direction Knockback%20Strength Knockback%20Strength%20Z))

(fn GuardStart
  (|CallParentFunction)
  (CallFunction|GuardStartEvent))

(fn GuardEnd
  (|CallParentFunction)
  (CallFunction|GuardEndEvent))