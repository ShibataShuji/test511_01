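; AI controller for enemy type 03 that runs behavior tree BT_03 on BeginPlay.
; Its AIPerception component reacts to target perception updates, filtering for the player character only.
; A successful sense writes the player to the TargetActor blackboard key, and a lost sense clears that key to null.
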(event OnTargetPerceptionUpdated(AIPerception)
  (params (Actor :type Actor%20Object%20Reference) (Stimulus :type AI%20Stimulus%20Structure))
  (if (== Actor (Game|GetPlayerCharacter 0))
    (if (.bSuccessfullySensed (Utilities|Struct|BreakAIStimulus Stimulus))
      ;[1 1 1] プレイヤーをセットする
      (AI|Components|Blackboard|SetValueasObject (Variables|Default|GetBlackboard) (Utilities|Name|MakeLiteralName "TargetActor") Actor)
      (else
        ;[1 1 1] nullをセットする
        (AI|Components|Blackboard|SetValueasObject (Variables|Default|GetBlackboard) (Utilities|Name|MakeLiteralName "TargetActor") 0)))))

(event EventBeginPlay
  (AI|RunBehaviorTree "/Game/MyContents/Enemy/03_Back/BT_03.BT_03"))

(event EventTick
  (params (DeltaSeconds :type Float%20%28single-precision%29)))

(fn ConstructionScript)