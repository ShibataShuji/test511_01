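; BP_AIEnemy_03_Back is an AI enemy that adds a shield guard on top of its parent enemy class.
; Guard Start and Guard End overrides switch the battle state and guard flag, spawning BP_Weapon_Shield in front of the enemy and destroying it afterwards.
; Knockback only calls the parent.
; An unconnected timeline holds a capsule trace that would knock back the player on contact, but it never runs.
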(event Custom|Guard%20End%20Event
  (Development|PrintString "ガード終了")
  (Variables|Default|SetBattleState "NewEnumerator0")
  (Variables|Default|SetOn%20Guard false)
  (bind _shieldactor (Variables|Default|GetShieldActor)
    (:then
      (Actor|DestroyActor _shieldactor))
    (:else)))

(event Custom|Guard%20Start%20Event
  (bind _returnvalue (Transformation|GetActorTransform))
  (bind (_location _rotation) (Math|Transform|BreakTransform _returnvalue))
  (Development|PrintString "ガード開始")
  (Variables|Default|SetBattleState "NewEnumerator3")
  (Variables|Default|SetOn%20Guard true)
  (bind _returnvalue_2 (Game|SpawnActorfromClass "/Game/MyContents/Weapon/Shield/BP_Weapon_Shield.BP_Weapon_Shield_C" (Math|Transform|MakeTransform (+ _location (* (Math|Vector|GetForwardVector _rotation) 5e+01)) _rotation) "AlwaysSpawn" 0 self 0))
  (Variables|Default|SetShieldActor _returnvalue_2))

(event EventBeginPlay
  (|CallParentFunction))

(event Collision|EventActorBeginOverlap
  (params (OtherActor :type Actor%20Object%20Reference)))

(event EventTick
  (params (DeltaSeconds :type Float%20%28single-precision%29)))

(fn ConstructionScript
  (|CallParentFunction))

(fn Knockback
  (params (Knockback%20Direction :type Vector :default "0, 0, 0") (Knockback%20Strength :type Float%20%28double-precision%29) (Knockback%20Strength%20Z :type Float%20%28double-precision%29))
  (|CallParentFunction Knockback%20Direction Knockback%20Strength Knockback%20Strength%20Z))

(fn GuardStart
  (|CallParentFunction)
  (CallFunction|GuardStartEvent))

(fn GuardEnd
  (|CallParentFunction)
  (CallFunction|GuardEndEvent))