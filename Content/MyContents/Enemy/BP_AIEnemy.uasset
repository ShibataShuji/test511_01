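; Base AI enemy character that saves its home location, supplies spline-based move locations, and leaves guard and target-detection actions as stubs, presumably for child classes.
; Knockback freezes the actor via CustomTimeDilation while a timer shakes the mesh with decaying amplitude, then restores time and activates the knockback gameplay ability granted on BeginPlay.
; A timeline eases rotation toward a target.
; The capsule-trace contact knockback on BP_Player is unconnected.
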(event Custom|Move%20Event
  (Variables|Default|GetMove%20Spline
    (:then
      (bind _spline_move_point (Default|GetSplineMoveLocation (Variables|Default|GetMove%20Spline)))
      (Variables|Default|SetMove%20Location _spline_move_point))
    (:else
      (Variables|Default|SetMove%20Location (Transformation|GetActorLocation)))))

(event Custom|Mesh%20Vibration
  (Variables|Default|SetMesh%20Vibration%20ElapsedTime 0.0)
  (Variables|Default|SetCustomTimeDilation 0.0)
  (bind _returnvalue (Utilities|Time|SetTimerbyEvent (delegate Custom|Mesh%20Vibration%20Sub1) (Variables|Default|GetMesh%20Vibration%20Interval%20Time) true))
  (Variables|Default|SetMesh%20Vibration%20Timer _returnvalue))

(event Custom|Mesh%20Vibration%20Sub1
  (bind _mesh_vibration_time (Variables|Default|GetMesh%20Vibration%20Time))
  (Variables|Default|SetMesh%20Vibration%20ElapsedTime (+ (Variables|Default|GetMesh%20Vibration%20ElapsedTime) (Class|KismetSystemLibrary|GetTimerElapsedTimeHandle (Variables|Default|GetMesh%20Vibration%20Timer))))
  (if (< (Variables|Default|GetMesh%20Vibration%20ElapsedTime) _mesh_vibration_time)
    (Utilities|FlowControl|FlipFlop
      (:A
        (Transformation|SetRelativeLocation (Variables|Character|GetMesh) (+ (Variables|Default|GetMesh%20Default%20Relative%20Location) (* (Variables|Ability|GetKnockback%20Direction) (Variables|Default|GetMesh%20Vibration%20Strength) (Math|Interpolation|Ease "Linear" (/ (Variables|Default|GetMesh%20Vibration%20ElapsedTime) _mesh_vibration_time) (Math|Float|MakeLiteralFloat 1.0) (Math|Float|MakeLiteralFloat 0.0)))) false true))
      (:B
        (Transformation|SetRelativeLocation (Variables|Character|GetMesh) (+ (Variables|Default|GetMesh%20Default%20Relative%20Location) (* (* (Variables|Ability|GetKnockback%20Direction) (Variables|Default|GetMesh%20Vibration%20Strength) (Math|Interpolation|Ease "Linear" (/ (Variables|Default|GetMesh%20Vibration%20ElapsedTime) _mesh_vibration_time) (Math|Float|MakeLiteralFloat 1.0) (Math|Float|MakeLiteralFloat 0.0))) -1.0)) false true)))
    (else
      (Transformation|SetRelativeLocation (Variables|Character|GetMesh) (Variables|Default|GetMesh%20Default%20Relative%20Location) false true)
      (Utilities|Time|ClearandInvalidateTimerbyHandle (Variables|Default|GetMesh%20Vibration%20Timer))
      (Variables|Default|SetCustomTimeDilation 1.0)
      (Abilities|TryActivateAbilitybyClass (Variables|Default|GetAbilitySystem) (Variables|Ability|GetKnockback%20Ability) true))))

(event Custom|Rotate%20toward%20the%20target%20Event
  (params (Target%20Location :type Vector))
  (bind _returnvalue (Transformation|GetActorLocation))
  (bind _returnvalue_2 (* Target%20Location "1.000000,1.000000,0.000000"))
  (bind _rotate_toward_the_target_time (Variables|Default|GetRotate%20toward%20the%20target%20Time))
  (bind _returnvalue_3 (* _returnvalue "1.000000,1.000000,0.000000"))
  (bind _returnvalue_4 (Math|Rotator|FindLookatRotation _returnvalue_3 _returnvalue_2))
  (Variables|Default|Settemp%20Rotation (Transformation|GetActorRotation))
  (bind _elapsed_time (Timeline|5sTimeline PlayFromStart)
    (:Update
      (if (> _elapsed_time _rotate_toward_the_target_time)
        (Transformation|SetActorRotation _returnvalue_4)
        (Timeline|5sTimeline Stop)
        (else
          (Transformation|SetActorRotation (Math|Interpolation|Ease "Linear" (/ _elapsed_time _rotate_toward_the_target_time) (Variables|Default|Gettemp%20Rotation) _returnvalue_4 true)))))))

(event EventBeginPlay
  (Utilities|FlowControl|Sequence
    (:then_0
      ;[1 1 1] 初期位置を保存しておく。ここに戻ったりする。
      (Variables|Default|SetHome%20Location (Transformation|GetActorLocation))
      (bind _move_spline (Variables|Default|GetMove%20Spline)
        (:then
          (Default|SetOwnerActor _move_spline self (* (Variables|/Script/Engine.CharacterMovementComponent|GetMaxWalkSpeed (Variables|Character|GetCharacterMovement)) 0.8)))
        (:else)))
    (:then_1
      (GameplayAbilities|GiveAbility (Variables|Default|GetAbilitySystem) (Variables|Ability|GetKnockback%20Ability) 0 -1))))

(fn ConstructionScript
  (Variables|Default|SetMesh%20Default%20Relative%20Location (Variables|/Script/Engine.SceneComponent|GetRelativeLocation (Variables|Character|GetMesh))))

(fn Knockback
  (params (Knockback%20Direction :type Vector) (Knockback%20Strength :type Float%20%28double-precision%29) (Knockback%20Strength%20Z :type Float%20%28double-precision%29))
  (Variables|Ability|SetKnockback%20Direction Knockback%20Direction)
  (Variables|Ability|SetKnockback%20Strength Knockback%20Strength)
  (Variables|Ability|SetKnockback%20Strength%20Z Knockback%20Strength%20Z)
  (CallFunction|MeshVibration))

(fn GuardStart)

(fn GuardEnd)

(fn ActionwhentheTargetIsNotinSight
  (return false))

(fn ActionattheMomentOfFindingtheTarget)

(fn ActiontobeTakenOutOfRange
  (return))

(fn ActiontobeTakenWithinRange)

(fn ActionattheMomentOfLoss)

(fn RotateTowardtheTarget
  (params (Target%20Location :type Vector))
  (CallFunction|RotateTowardtheTargetEvent Target%20Location))