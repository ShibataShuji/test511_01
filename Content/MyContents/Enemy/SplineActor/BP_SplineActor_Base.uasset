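; Base spline path actor for enemies, providing a moving world location for an owner actor through GetSplineMoveLocation.
; SetOwnerActor stores owner and speed, deriving travel time from spline length.
; A timeline named 100sTimeline serves as a clock, reversing past travel time and restarting on finish to ping-pong the sampled constant-velocity point and Sphere along the spline.
; A second timeline delays a check that prints a warning if no valid owner is set.
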(event Custom|Check%20Owner%20Actor
  (Timeline|タイムライン PlayFromStart
    (:Finished
      (Variables|Default|GetOwner%20Actor
        (:then)
        (:else
          (Development|PrintString (Utilities|String|Append (Utilities|String|MakeLiteralString (Utilities|GetObjectName self)) (Utilities|String|MakeLiteralString "有効なオーナーとなるアクターがセットされていません"))))))))

(event Custom|Update%20Spline%20Point%20Location
  ;[1 1 1] 生き返りの往復処理
  (bind _elapsed_time (Timeline|100sTimeline Play)
    (:Update
      (if (> _elapsed_time (Variables|Default|GetTime%20it%20takes))
        (Utilities|FlowControl|Sequence
          (:then_0
            (Timeline|100sTimeline Reverse))
          (:then_1
            (Variables|Default|SetSpline%20Move%20Location (Spline|GetLocationatTime (Variables|Default|GetSpline) (/ _elapsed_time (Variables|Default|GetTime%20it%20takes)) "World" true) :!label _label)
            (Transformation|SetWorldLocation (Variables|Default|GetSphere) (Spline|GetLocationatTime (Variables|Default|GetSpline) (/ _elapsed_time (Variables|Default|GetTime%20it%20takes)) "World" true) false false)))
        (else
          (goto _label))))
    (:Finished
      (Timeline|100sTimeline PlayFromStart))))

(event EventBeginPlay
  (CallFunction|CheckOwnerActor)
  (CallFunction|UpdateSplinePointLocation))

(fn ConstructionScript)

(fn SetOwnerActor
  (params (Owner%20Actor :type Actor%20Object%20Reference) (Owner%20Move%20Speed :type Float%20%28double-precision%29))
  (Variables|Default|SetOwner%20Actor Owner%20Actor)
  (Variables|Default|SetOwner%20Move%20Speed Owner%20Move%20Speed)
  (Variables|Default|SetTime%20it%20takes (/ (Spline|GetSplineLength (Variables|Default|GetSpline)) (Variables|Default|GetOwner%20Move%20Speed))))

(fn GetSplineMoveLocation
  (return (Variables|Default|GetSpline%20Move%20Location)))