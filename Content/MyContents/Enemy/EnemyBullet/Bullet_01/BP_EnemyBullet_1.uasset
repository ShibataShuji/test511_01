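; BP_EnemyBullet_1 is an enemy projectile that expires after its LifeTime.
; On overlapping the player, it reports the hit to its valid owner enemy through HitPlayer, passing its forward vector and hit strength.
; The HitBullet override calls the parent and fires an event marked for reflection, which only prints a debug string.
; Homing setup nodes exist but are never run.
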(event Custom|Hit%20Bullet%20Event
  (Development|PrintString "aaaaaaaaaaaaaaaaaaaaaaaaaaaaaaaa"))

(event EventBeginPlay
  (Actor|SetLifeSpan (Variables|Default|GetLifeTime)))

(event Collision|EventActorBeginOverlap
  (params (OtherActor :type Actor%20Object%20Reference))
  (Utilities|FlowControl|Sequence
    (:then_0
      ;[1 1 1] プレイヤーに当たったよ
      (if (.bSuccess (Utilities|Casting|CastToBP_Player OtherActor))
        (bind _ownerenemy (Variables|Default|GetOwnerEnemy)
          (:then
            (Default|HitPlayer _ownerenemy (Transformation|GetActorForwardVector) (Variables|Default|GetHitStrangth)))
          (:else))))))

(event EventTick
  (params (DeltaSeconds :type Float%20%28single-precision%29)))

(fn ConstructionScript
  (|CallParentFunction))

(fn HitBullet
  (|CallParentFunction)
  (CallFunction|HitBulletEvent))