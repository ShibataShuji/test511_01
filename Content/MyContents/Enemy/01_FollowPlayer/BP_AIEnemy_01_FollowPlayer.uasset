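; Follow-player enemy Blueprint that knocks the player back on contact.
; From BeginPlay, a timeline's Update runs an object-type capsule trace at the enemy's position, slightly larger than its capsule, with debug drawing on.
; A hit on BP_Player calls that player's Knockback, directed away from the enemy.
; The enemy's own Knockback only forwards to the parent, and no follow movement is defined here.
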(event EventBeginPlay
  (bind _capsulecomponent (Variables|Default|GetCapsuleComponent))
  (bind (_outradius _outhalfheight) (Components|Capsule|GetScaledCapsuleSize _capsulecomponent))
  (bind _returnvalue (Transformation|GetWorldLocation _capsulecomponent))
  (|CallParentFunction)
  (Timeline|タイムライン_0 PlayFromStart
    (:Update
      (bind (_outhit _returnvalue_2) (Class|KismetSystemLibrary|CapsuleTraceSingleforObjects _returnvalue _returnvalue (* _outradius 1.1) (* _outhalfheight 1.1) (Variables|Default|GetObject%20Types) false 0 "ForOneFrame" true))
      (if _returnvalue_2
        (if (.bSuccess (Utilities|Casting|CastToBP_Player (.HitActor (Collision|BreakHitResult _outhit))))
          (Default|Knockback (.AsBP%20Player (Utilities|Casting|CastToBP_Player (.HitActor (Collision|BreakHitResult _outhit)))) (Math|Vector|Normalize (- (Transformation|GetActorLocation (.HitActor (Collision|BreakHitResult _outhit))) (Transformation|GetActorLocation))) 8e+02 0.1))))))

(event Collision|EventActorBeginOverlap
  (params (OtherActor :type Actor%20Object%20Reference)))

(event EventTick
  (params (DeltaSeconds :type Float%20%28single-precision%29)))

(fn ConstructionScript
  (|CallParentFunction))

(fn Knockback
  (params (Knockback%20Direction :type Vector :default "0, 0, 0") (Knockback%20Strength :type Float%20%28double-precision%29) (Knockback%20Strength%20Z :type Float%20%28double-precision%29))
  (|CallParentFunction Knockback%20Direction Knockback%20Strength Knockback%20Strength%20Z))