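; GA_Knockback is a gameplay ability that sets up a knockback on its avatar, either a BP_AIEnemy or a BP_Player.
; On activation it builds Direction from the avatar's KnockbackDirection plus an upward component.
; Enemies use their own KnockbackStrengthZ and KnockbackStrength, while the player uses the ability's KnockUp and leaves Strength untouched.
; It then calls the parent's activation and also prints the avatar's name.
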(event Ability|EventActivateAbility
  (bind _returnvalue (Ability|GetAvatarActorfromActorInfo))
  (bind _returnvalue_2 (Ability|GetAvatarActorfromActorInfo))
  (bind (_asbp_player _bsuccess) (Utilities|Casting|CastToBP_Player _returnvalue))
  (bind (_asbp_aienemy _bsuccess_2) (Utilities|Casting|CastToBP_AIEnemy _returnvalue_2))
  (Utilities|FlowControl|Sequence
    (:then_0
      (Development|PrintString (Utilities|GetDisplayName (Ability|GetAvatarActorfromActorInfo)))
      (if _bsuccess_2
        (Variables|Default|SetDirection (+ (Variables|/Game/MyContents/Enemy/BP_AIEnemy.BP_AIEnemy_C|GetKnockback%20Direction _asbp_aienemy) (* (Transformation|GetActorUpVector _returnvalue_2) (Variables|/Game/MyContents/Enemy/BP_AIEnemy.BP_AIEnemy_C|GetKnockback%20Strength%20Z _asbp_aienemy))))
        (Variables|Default|SetStrength (Variables|/Game/MyContents/Enemy/BP_AIEnemy.BP_AIEnemy_C|GetKnockback%20Strength _asbp_aienemy))
        (|CallParentFunction)))
    (:then_1
      (if _bsuccess
        (Variables|Default|SetDirection (+ (Variables|/Game/MyContents/Player/BP_Player.BP_Player_C|GetKnockback%20Direction _asbp_player) (* (Transformation|GetActorUpVector _returnvalue) (Variables|Default|GetKnockUp))))
        (|CallParentFunction)))))

(event Ability|EventOnEndAbility
  (params (bWasCancelled :type Boolean))
  (|CallParentFunction bWasCancelled) ; このノードは無効になっているため呼び出せません。\n機能をビルドするにはピンをドラッグしてください。
)