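; BP_Weapon_Shield is a shield weapon actor that positions itself in front of its owning enemy while that enemy guards.
; After the parent BeginPlay, it starts a timeline if OwnerEnemy is valid, using the timeline's Update in place of Tick.
; Each update with OnGuard set snaps the shield a fixed distance along the enemy's forward vector, matching its rotation at unit scale.
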(event EventBeginPlay
  (|CallParentFunction)
  (bind _owner_enemy (Variables|Default|GetOwner%20Enemy)
    (:then
      (Timeline|タイムライン_0 PlayFromStart
        (:Update
          (if (Variables|/Game/MyContents/Enemy/BP_AIEnemy.BP_AIEnemy_C|GetOn%20Guard (Variables|Default|GetOwner%20Enemy))
            (Transformation|SetActorTransform (Math|Transform|MakeTransform (+ (.Location (Math|Transform|BreakTransform (Transformation|GetActorTransform _owner_enemy))) (* (Math|Vector|GetForwardVector (.Rotation (Math|Transform|BreakTransform (Transformation|GetActorTransform _owner_enemy)))) 5e+01)) (.Rotation (Math|Transform|BreakTransform (Transformation|GetActorTransform _owner_enemy)))))))))
    (:else)))

(event Collision|EventActorBeginOverlap
  (params (OtherActor :type Actor%20Object%20Reference))
  (|CallParentFunction OtherActor) ; このノードは無効になっているため呼び出せません。\n機能をビルドするにはピンをドラッグしてください。
)

(event EventTick
  (params (DeltaSeconds :type Float%20%28single-precision%29))
  (|CallParentFunction DeltaSeconds) ; このノードは無効になっているため呼び出せません。\n機能をビルドするにはピンをドラッグしてください。
)

(fn ConstructionScript
  (|CallParentFunction))