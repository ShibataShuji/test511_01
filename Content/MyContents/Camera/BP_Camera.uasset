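; BP_Camera is the main spring-arm camera actor, which follows the player character and registers itself with BP_Player on BeginPlay.
; Each Tick it moves to the target plus a height offset, applying arm length, arm direction and camera pitch from its variables.
; It exposes camera forward and right vectors, optionally flattened on Z, and UseCamera makes it the view target.
; A timeline-driven attention-point zoom and return exists but is disconnected, leaving AttentionPoint empty.
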(event Custom|Follow%20Target
  (CallFunction|CameraLocationUpdate))

(event Custom|Use%20Camera
  (Game|Player|SetViewTargetwithBlend (Game|GetPlayerController 0) self 0.0 "VTBlend_Linear" 0.0 false))

(event Custom|Attention%20Point
  (params (Attention%20Location :type Vector)))

(event Custom|Attention%20Point%20Sub1)

(event Custom|Camera%20Location%20Update
  (Variables|/Script/Engine.SpringArmComponent|SetTargetArmLength (Variables|Default|GetSpringArm) (Variables|Default|GetLength%20to%20Target))
  (Transformation|SetRelativeRotation (Variables|Default|GetSpringArm) (Variables|Default|GetDirection%20to%20Target) false false)
  (Transformation|SetActorLocation (+ (Utilities|Select :Index (Variables|Default|GetCamera%20Mode) :NewEnumerator0 (Transformation|GetActorLocation (Variables|Default|GetTarget%20Actor)) :NewEnumerator1 (Variables|Default|GetAttention%20Location)) (Math|Vector|MakeVector 0.0 0.0 (Variables|Default|GetOffset%20Height))) false false)
  (Transformation|SetRelativeRotation (Variables|Default|GetCamera) (Math|Rotator|MakeRotator 0.0 (Variables|Default|GetRotate%20Yaw%20to%20Target) 0.0) false false))

(event EventBeginPlay
  (bind _returnvalue (Game|GetPlayerCharacter 0))
  (bind (_asbp_player _bsuccess) (Utilities|Casting|CastToBP_Player _returnvalue))
  (Utilities|FlowControl|Sequence
    (:then_0
      (Variables|Default|SetTarget%20Actor _returnvalue)
      (if _bsuccess
        (Default|SetMainCameraActor _asbp_player self)))))

(event Collision|EventActorBeginOverlap
  (params (OtherActor :type Actor%20Object%20Reference)))

(event EventTick
  (params (DeltaSeconds :type Float%20%28single-precision%29))
  (Variables|Default|GetTarget%20Actor
    (:then
      (if (Utilities|Enum|Equal(Enum) (Variables|Default|GetCamera%20Mode) "NewEnumerator0")
        _
        (else
          _))
      (CallFunction|FollowTarget))
    (:else
      (Development|PrintString "カメラのターゲットアクターがないよ"))))

(fn ConstructionScript
  ;[1 1 1] Actorの回転は使わない。
  (Transformation|SetActorRotation "0, 0, 0")
  (Variables|Default|SetDef%20Length%20To%20Target (Variables|Default|GetLength%20to%20Target))
  (Variables|Default|SetDef%20Offset%20Height (Variables|Default|GetOffset%20Height)))

(fn GetCameraForward
  (return (Math|Vector|GetForwardVector (Variables|Default|GetCamera))))

(fn GetCameraRight
  (return (Math|Vector|GetRightVector (Variables|Default|GetCamera))))

(fn GetCameraForwardIgnoreZ
  (return (Math|Vector|Normalize (* (Math|Vector|GetForwardVector (Variables|Default|GetCamera)) "1.000000,1.000000,0.000000"))))

(fn GetCameraRightIgnoreZ
  (return (Math|Vector|Normalize (* (Math|Vector|GetRightVector (Variables|Default|GetCamera)) "1.000000,1.000000,0.000000"))))